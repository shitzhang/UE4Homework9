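; Grenade projectile Blueprint whose event graph is inactive: BeginPlay is empty and the construction script does nothing.
; Two disconnected node chains remain, one calling Explode after a short delay.
; The other holds explosion logic that never runs: particle effect, full radial damage and impulse sized by RadialForceComp, debug sphere, then actor destruction.
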(event EventBeginPlay)

(fn ConstructionScript)