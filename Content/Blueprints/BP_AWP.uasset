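; AWP sniper weapon Blueprint that shows a scope overlay and zooms the view while targeting.
; It creates the sniper HUD widget once at BeginPlay, then adds it to the viewport behind other widgets on StartTarget.
; Targeting also narrows the TargetingFOV on the local ShooterPlayerCameraManager.
; Ending targeting, unequipping or destruction share one cleanup path that removes the overlay and widens that FOV again.
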(event EventBeginPlay
  (bind _returnvalue (UserInterface|CreateWidget "/Game/UI/WBP_SniperHUD.WBP_SniperHUD_C"))
  (Variables|Default|SetSniperHUD _returnvalue))

(event EventDestroyed
  (bind _returnvalue (Game|GetPlayerController 0))
  (bind _sniperhud (Variables|Default|GetSniperHUD))
  (Utilities|IsValid _sniperhud
    (:Is%20Valid
      (Widget|RemovefromParent _sniperhud)
      (Utilities|IsValid _returnvalue
        (:Is%20Valid
          (bind _asshooter_player_camera_manager (Utilities|Casting|CastToShooterPlayerCameraManager (Variables|/Script/Engine.PlayerController|GetPlayerCameraManager _returnvalue)))
          (Variables|/Script/prototype.ShooterPlayerCameraManager|SetTargetingFOV _asshooter_player_camera_manager 65.0))))))

(event EventOnUnEquip
  (bind _returnvalue (Game|GetPlayerController 0))
  (bind _sniperhud (Variables|Default|GetSniperHUD))
  (Utilities|IsValid _sniperhud
    (:Is%20Valid
      (Widget|RemovefromParent _sniperhud)
      (Utilities|IsValid _returnvalue
        (:Is%20Valid
          (bind _asshooter_player_camera_manager (Utilities|Casting|CastToShooterPlayerCameraManager (Variables|/Script/Engine.PlayerController|GetPlayerCameraManager _returnvalue)))
          (Variables|/Script/prototype.ShooterPlayerCameraManager|SetTargetingFOV _asshooter_player_camera_manager 65.0))))))

(event EventStartTarget
  (bind _returnvalue (Game|GetPlayerController 0))
  (bind _sniperhud (Variables|Default|GetSniperHUD))
  (Utilities|IsValid _sniperhud
    (:Is%20Valid
      (UserInterface|Viewport|AddtoViewport _sniperhud -15)
      (Utilities|IsValid _returnvalue
        (:Is%20Valid
          (bind _asshooter_player_camera_manager (Utilities|Casting|CastToShooterPlayerCameraManager (Variables|/Script/Engine.PlayerController|GetPlayerCameraManager _returnvalue)))
          (Variables|/Script/prototype.ShooterPlayerCameraManager|SetTargetingFOV _asshooter_player_camera_manager 15.0))))))

(event EventEndTarget
  (bind _returnvalue (Game|GetPlayerController 0))
  (bind _sniperhud (Variables|Default|GetSniperHUD))
  (Utilities|IsValid _sniperhud
    (:Is%20Valid
      (Widget|RemovefromParent _sniperhud)
      (Utilities|IsValid _returnvalue
        (:Is%20Valid
          (bind _asshooter_player_camera_manager (Utilities|Casting|CastToShooterPlayerCameraManager (Variables|/Script/Engine.PlayerController|GetPlayerCameraManager _returnvalue)))
          (Variables|/Script/prototype.ShooterPlayerCameraManager|SetTargetingFOV _asshooter_player_camera_manager 65.0))))))

(fn ConstructionScript)